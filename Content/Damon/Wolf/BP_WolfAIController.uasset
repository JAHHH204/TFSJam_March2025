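; BP_WolfAIController is the AI controller for the wolf, wandering it around its den or chasing the player.
; BeginPlay caches the den actor's location, and wandering moves to random navigable points near it, setting a looping timer on arrival.
; Tick chases the player when CanSeePlayer is true, otherwise re-issues the wander every frame.
; LookForPlayer is unfinished: it loops over sight-perceived actors with an empty body, and nothing here sets CanSeePlayer.
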(event Custom|WanderAroundDen
  (bind _randomlocation (Class|NavigationSystemV1|GetRandomLocationinNavigableRadius (Variables|Default|GetDenLocation) 5e+02 0 0))
  (bind _asbp_wolf_ai (Utilities|Casting|CastToBP_WolfAI (Pawn|GetControlledPawn self)))
  (AI|AIMoveTo _asbp_wolf_ai _randomlocation 0 5.0 false
    (:OnSuccess
      (Utilities|Time|SetTimerbyFunctionName 0 "WanderAroundDen" 1.0 true))))

(event Custom|LookForPlayer
  (bind _asbp_wolf_ai (Utilities|Casting|CastToBP_WolfAI (Pawn|GetControlledPawn)))
  (for _array_element (Class|AIPerceptionComponent|GetCurrentlyPerceivedActors (Variables|/Game/Damon/Wolf/BP_WolfAI.BP_WolfAI_C|GetAIPerception _asbp_wolf_ai) "/Script/AIModule.AISense_Sight")
    _))

(event EventBeginPlay
  (bind _asbp_wolf_ai (Utilities|Casting|CastToBP_WolfAI (Pawn|GetControlledPawn)))
  (Variables|Default|SetDenLocation (Transformation|GetActorLocation (Variables|/Game/Damon/Wolf/BP_WolfAI.BP_WolfAI_C|GetDenActor _asbp_wolf_ai)))
  (CallFunction|WanderAroundDen))

(event EventTick
  (params (DeltaSeconds :type Float%20%28single-precision%29))
  (if (Variables|Default|GetCanSeePlayer)
    (AI|AIMoveTo (Pawn|GetControlledPawn self) "0, 0, 0" (Game|Player|GetPlayerPawn 0) 5.0 false)
    (else
      (CallFunction|WanderAroundDen))))

(fn ConstructionScript)