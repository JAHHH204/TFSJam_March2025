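; AI controller for a bear that wanders around its den and attacks beaver players it sees.
; Without a behavior tree, it uses boolean flags and a delay-throttled Tick to poll the pawn's AIPerception sight while not chasing.
; With no beaver visible, AIMoveTo sends it to random navigable points near DenActor.
; A sighted beaver becomes the chase target, taking damage when reached, and either move outcome ends the chase.
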(event Custom|WanderAroundDen
  (bind _randomlocation (Class|NavigationSystemV1|GetRandomLocationinNavigableRadius (Variables|Default|GetDenLocation) 5e+02 0 0))
  (bind _asbp_bear_ai (Utilities|Casting|CastToBP_BearAI (Pawn|GetControlledPawn self)))
  (AI|AIMoveTo _asbp_bear_ai _randomlocation 0 5.0 false
    (:OnSuccess
      (Variables|Default|SetIsWandering false))))

(event Custom|LookForPlayer
  (bind _asbp_bear_ai (Utilities|Casting|CastToBP_BearAI (Pawn|GetControlledPawn)))
  (bind _array_element (Utilities|Array|ForEachLoopwithBreak (Class|AIPerceptionComponent|GetCurrentlyPerceivedActors (Variables|/Game/Damon/Bear/BP_BearAI.BP_BearAI_C|GetAIPerception _asbp_bear_ai) "/Script/AIModule.AISense_Sight") :!label _label)
    (:LoopBody
      (bind _asbp_beaver (Utilities|Casting|CastToBP_Beaver _array_element)
        (:then
          (Variables|Default|SetCurrentTarget _asbp_beaver)
          (Variables|Default|SetCanSeePlayer true)
          (Variables|Default|SetIsWandering false)
          (goto _label Break))
        (:CastFailed
          (Variables|Default|SetCurrentTarget 0)
          (Variables|Default|SetCanSeePlayer false))))
    (:Completed
      (if (Variables|Default|GetCanSeePlayer)
        (Variables|Default|SetIsChasing true)
        (CallFunction|ChasePlayer)
        (elif (not (Variables|Default|GetIsWandering))
          (Variables|Default|SetIsWandering true)
          (CallFunction|WanderAroundDen))))))

(event Custom|ChasePlayer
  (AI|AIMoveTo (Pawn|GetControlledPawn) "0, 0, 0" (Variables|Default|GetCurrentTarget) 7.0 false
    (:OnSuccess
      (Game|Damage|ApplyDamage (Variables|Default|GetCurrentTarget) 1.0 0 0))
    (:OnFail
      _))
  (Variables|Default|SetIsChasing false)
  (Variables|Default|SetCanSeePlayer false))

(event EventBeginPlay
  (bind _asbp_bear_ai (Utilities|Casting|CastToBP_BearAI (Pawn|GetControlledPawn)))
  (Variables|Default|SetDenLocation (Transformation|GetActorLocation (Variables|/Game/Damon/Bear/BP_BearAI.BP_BearAI_C|GetDenActor _asbp_bear_ai)))
  (CallFunction|WanderAroundDen))

(event EventTick
  (params (DeltaSeconds :type Float%20%28single-precision%29))
  (Utilities|FlowControl|Delay 0.2)
  (if (not (Variables|Default|GetIsChasing))
    (CallFunction|LookforPlayer)))

(fn ConstructionScript)