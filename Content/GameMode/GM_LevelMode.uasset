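; Level game mode that tracks a log-collection objective scaled to the number of players.
; Starting the game stores the player count and sets the log target from a fixed lookup for one to four players.
; Collecting a log increments a counter, with no comparison against the target in this graph.
; Both actions enter through Server-named events that forward to a second event, which calls the function doing the work.
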(event Custom|Start%20Game%20Event
  (params (Number%20of%20Players :type Integer))
  ;[1 1 1] Start Actual Game events
  (CallFunction|StartGameFunction Number%20of%20Players))

(event Custom|Collect%20Log%20Server%20Event
  ;[1 1 1] Dont touch my log you dirty boys
  (CallFunction|CollectLogEvent))

(event Custom|Start%20Game%20Server%20Event
  (params (Number%20of%20Players :type Integer))
  ;[1 1 1] Start Actual Game events
  (CallFunction|StartGameEvent Number%20of%20Players))

(event Custom|Collect%20Log%20Event
  ;[1 1 1] Dont touch my log you dirty boys
  (CallFunction|CollectLogFunction))

(event EventBeginPlay)

(event EventTick
  (params (DeltaSeconds :type Float%20%28single-precision%29)))

(fn ConstructionScript)

(fn StartGameFunction
  (params (Number%20of%20Players :type Integer))
  (bind _output_get (Variables|Default|SetNumber%20of%20Players Number%20of%20Players))
  (switch int _output_get
    (:1
      (Variables|Default|SetLogs%20To%20Collect 16))
    (:2
      (Variables|Default|SetLogs%20To%20Collect 24))
    (:3
      (Variables|Default|SetLogs%20To%20Collect 36))
    (:4
      (Variables|Default|SetLogs%20To%20Collect 40))))

(fn CollectLogFunction
  (Variables|Default|SetLogs%20Collected (+ (Variables|Default|GetLogs%20Collected) 1)))