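; Base tree actor that players chop down by damage and then drag, with speed penalties.
; At zero health it enables physics and gets pushed at its top along the damage causer's forward vector, freezing once Tick sees it settle.
; Dragging re-enables physics and slows each player, splitting the penalty among all draggers, until the last one leaves.
; RPC-named events re-apply the body's current transform.
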(event Custom|RPC_Server_TrackLocation
  (CallFunction|RPCTrackLocation))

(event Custom|RPC_TrackLocation
  (bind _treebody (Variables|Default|GetTreeBody))
  (Transformation|SetWorldLocationAndRotation (Variables|Default|GetTreeBody) (Transformation|GetWorldLocation _treebody) (Transformation|GetWorldRotation _treebody) false false))

(event Custom|OnTakeAnyDamage_Event
  (params (DamagedActor :type Actor%20Object%20Reference) (Damage :type Float%20%28single-precision%29) (DamageType :type Damage%20Type%20Object%20Reference) (InstigatedBy :type Controller%20Object%20Reference) (DamageCauser :type Actor%20Object%20Reference))
  (if (not (Variables|Default|GetChoppedDown))
    (bind _output_get (Variables|Default|SetHealth (- (Variables|Default|GetHealth) Damage)))
    (if (<= _output_get 0.0)
      (Variables|Default|SetChoppedDown true)
      (Variables|Default|SetHealth 0.0)
      (CallFunction|FellTree DamageCauser)
      (Utilities|FlowControl|Delay 0.5)
      (Variables|Default|SetFalling true))))

(event EventBeginPlay
  (Class|PrimitiveComponent|SetMassOverrideinKg (Variables|Default|GetTreeBody) "None" (Variables|Default|GetWeight) true)
  (EventDispatchers|AssignOnTakeAnyDamage (delegate Custom|OnTakeAnyDamage_Event)))

(event EventTick
  (params (DeltaSeconds :type Float%20%28single-precision%29))
  (if (Variables|Default|GetFalling)
    (if (<= (Math|Vector|VectorLength (Transformation|GetComponentVelocity (Variables|Default|GetTreeBody))) 0.2)
      (Variables|Default|SetFalling false)
      (Physics|SetSimulatePhysics (Variables|Default|GetTreeBody) false))))

(fn ConstructionScript)

(fn FellTree
  (params (ChoppingActor :type Actor%20Object%20Reference))
  (bind _treebody (Variables|Default|GetTreeBody))
  (Physics|SetSimulatePhysics (Variables|Default|GetTreeBody) true)
  (Physics|AddImpulseatLocation _treebody (* (Transformation|GetActorForwardVector ChoppingActor) (Variables|Default|GetFallForce)) (+ (Transformation|GetWorldLocation _treebody) (Math|Vector|MakeVector 0.0 0.0 (.z (.Max (Components|StaticMesh|GetLocalBounds _treebody))))) "None"))

(fn SlowdownPlayer
  (bind _playersdragging (Variables|Default|GetPlayersDragging))
  (bind _playersdragging_2 (Variables|Default|GetPlayersDragging))
  (bind _returnvalue (Utilities|Array|Length _playersdragging))
  (bind _output (Utilities|Array|Get(acopy) _playersdragging_2))
  (if (> _returnvalue 1)
    (for _array_element (Variables|Default|GetPlayersDragging)
      (Variables|/Script/Engine.CharacterMovementComponent|SetMaxWalkSpeed (Variables|/Script/Engine.Character|GetCharacterMovement _array_element) (- (Variables|/Game/PlayerController/BP_Beaver.BP_Beaver_C|GetBaseWalkSpeed _array_element) (/ (Variables|Default|GetSlowSpeedAmount) _returnvalue))))
    (else
      (Variables|/Script/Engine.CharacterMovementComponent|SetMaxWalkSpeed (Variables|/Script/Engine.Character|GetCharacterMovement _output) (- (Variables|/Game/PlayerController/BP_Beaver.BP_Beaver_C|GetBaseWalkSpeed _output) (Variables|Default|GetSlowSpeedAmount))))))

(fn AddPlayerDragging
  (params (Player :type BP%20Beaver%20Object%20Reference))
  (Utilities|Array|AddUnique (Variables|Default|GetPlayersDragging) Player)
  (CallFunction|SlowdownPlayer)
  (Physics|SetSimulatePhysics (Variables|Default|GetTreeBody) true))

(fn RemovePlayerDragging
  (params (Player :type BP%20Beaver%20Object%20Reference))
  (Utilities|Array|RemoveItem (Variables|Default|GetPlayersDragging) Player)
  (if (> (Utilities|Array|Length (Variables|Default|GetPlayersDragging)) 0)
    (CallFunction|SlowdownPlayer)
    (else
      (Physics|SetSimulatePhysics (Variables|Default|GetTreeBody) false))))