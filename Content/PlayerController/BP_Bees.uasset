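; BP_Bees is a short-lived bee actor that appears intended to chase the player, then destroys itself after a three-second delay.
; BeginPlay issues one AI MoveTo using player location minus its own, an offset rather than a world position, with a beaver reference cleared to None beforehand.
; Tick caches the player controller's location, which does not update the issued move.
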(event Custom|MoveToward
  (bind _output_get (Variables|Default|SetAs%20BP%20Beaver 0))
  (AI|AIMoveTo _output_get 0 (- (stale Custom|GetPos _output_get) (Transformation|GetActorLocation)) _output_get 5.0 false
    (:then
      _)
    (:OnSuccess
      _)
    (:OnFail
      _))
  (Utilities|FlowControl|Delay 3.0)
  (Actor|DestroyActor))

(event Custom|GetPos
  (bind _output_get (Variables|Default|SetPlayer%20Location (Transformation|GetActorLocation (Game|GetPlayerController 0)))))

(event EventTick
  (params (DeltaSeconds :type Float%20%28single-precision%29))
  (CallFunction|GetPos))

(event Collision|EventActorBeginOverlap
  (params (OtherActor :type Actor%20Object%20Reference)))

(event EventBeginPlay
  (CallFunction|MoveToward))

(fn ConstructionScript)