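; Component that lets a BP_Beaver player grab and drag chopped-down trees with the interact input.
; A lowered forward line trace finds the log, then a Physics Handle created at BeginPlay grabs it and the tree registers the dragging player.
; While dragging, Tick moves the handle target ahead of the beaver through server RPCs relayed to paired RPC events.
; Releasing the input drops the log, unregisters the player and restores base walk speed.
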(event Custom|RPC_DragLog
  (params (ObjectLocation :type Vector) (ObjectRotation :type Rotator))
  (Class|PhysicsHandleComponent|SetTargetLocationandRotation (Variables|Default|GetPhysicsHandleRef) ObjectLocation ObjectRotation))

(event Custom|RPC_Server_DragLog
  (bind _returnvalue (Components|GetOwner))
  (bind _physicshandleref (Variables|Default|GetPhysicsHandleRef))
  (bind (_targetlocation _targetrotation) (Class|PhysicsHandleComponent|GetTargetLocationandRotation _physicshandleref))
  (Physics|Components|PhysicsHandle|SetTargetLocation _physicshandleref (+ (- (Transformation|GetActorLocation _returnvalue) "0.000000,0.000000,75.000000") (* (Transformation|GetActorForwardVector _returnvalue) (Variables|Default|GetPullRange))))
  (CallFunction|RPCDragLog _targetlocation _targetrotation))

(event Custom|RPC_Server_GrabLog
  (CallFunction|RPCGrabLog))

(event Custom|RPC_GrabLog
  (bind (_loghit _logref _hit_location) (CallFunction|LineTrace))
  (if _loghit
    (bind _output_get (Variables|Default|SetTargetRef _logref))
    (bind _output_get_2 (Variables|Default|SetHitLocationRef _hit_location))
    (Variables|Default|SetIsDragging true)
    (Class|PhysicsHandleComponent|GrabComponentatLocation (Variables|Default|GetPhysicsHandleRef) _output_get "None" _output_get_2)
    (Default|AddPlayerDragging (Variables|Default|GetTreeRef) (Variables|Default|GetOwnerPlayerRef))))

(event Custom|RPC_Server_DropLog
  (CallFunction|RPCDropLog))

(event Custom|RPC_DropLog
  (bind _treeref (Variables|Default|GetTreeRef))
  (bind _ownerplayerref (Variables|Default|GetOwnerPlayerRef))
  (Physics|Components|PhysicsHandle|ReleaseComponent (Variables|Default|GetPhysicsHandleRef))
  (Variables|Default|SetTargetRef 0)
  (Variables|Default|SetIsDragging false)
  (Variables|Default|SetHitLocationRef "0, 0, 0")
  (Utilities|IsValid _treeref
    (:Is%20Valid
      (Default|RemovePlayerDragging _treeref _ownerplayerref)
      (Variables|/Script/Engine.CharacterMovementComponent|SetMaxWalkSpeed (Variables|/Script/Engine.Character|GetCharacterMovement _ownerplayerref) (Variables|/Game/PlayerController/BP_Beaver.BP_Beaver_C|GetBaseWalkSpeed _ownerplayerref)))))

(event Input|EnhancedActionEvents|EnhancedInputActionIA_Interact
  (params (ActionValue :type Boolean) (ElapsedSeconds :type Float%20%28double-precision%29) (TriggeredSeconds :type Float%20%28double-precision%29) (InputAction :type Input%20Action%20Object%20Reference :default "/Game/PlayerController/InputActions/IA_Interact.IA_Interact"))
  (:Started
    (CallFunction|RPCServerGrabLog))
  (:Canceled
    (CallFunction|RPCServerDropLog :!label _label))
  (:Completed
    (goto _label)))

(event EventBeginPlay
  (bind _returnvalue (Game|AddComponentbyClass (Components|GetOwner) "/Script/Engine.PhysicsHandleComponent"))
  (bind _output_get (Variables|Default|SetPhysicsHandleRef _returnvalue))
  (Class|PhysicsHandleComponent|SetInterpolationSpeed _output_get 7.5)
  (bind _asbp_beaver (Utilities|Casting|CastToBP_Beaver (Components|GetOwner)))
  (Variables|Default|SetOwnerPlayerRef _asbp_beaver))

(event EventTick
  (params (DeltaSeconds :type Float%20%28single-precision%29))
  (if (Variables|Default|GetIsDragging)
    (CallFunction|RPCServerDragLog)))

(fn LineTrace
  (bind _returnvalue (Components|GetOwner))
  (bind _returnvalue_2 (Transformation|GetActorLocation _returnvalue))
  (bind _returnvalue_3 (- _returnvalue_2 "0.000000,0.000000,75.000000"))
  (bind _outhit (Collision|LineTraceByChannel _returnvalue_3 (+ _returnvalue_3 (* (Transformation|GetActorForwardVector _returnvalue) (Variables|Default|GetPullRange))) "TraceTypeQuery1" false 0 "ForDuration"))
  (bind _asbp_base_tree (Utilities|Casting|CastToBP_BaseTree (.hitactor _outhit))
    (:then
      (if (Variables|/Game/Trees/BP_BaseTree.BP_BaseTree_C|GetChoppedDown _asbp_base_tree)
        (Variables|Default|SetTreeRef _asbp_base_tree)
        (return true (.hitcomponent _outhit) (.location _outhit))
        (else
          _)))
    (:CastFailed
      _))
  (return false 0 "0, 0, 0"))