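; AC_Chopper is an actor component that lets the beaver bite trees to chop them.
; IA_Bite input, gated by a one-second cooldown, calls a server-named RPC that runs the chop and plays the bite animation on player 0's character before restoring the looping one.
; The chop line-traces forward from the owner with debug drawing, damaging any hit BP_BaseTree and spawning a BP_Chip at the impact.
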(event Custom|RPC_Server_Chop
  (bind _returnvalue (Game|GetPlayerCharacter 0))
  (bind _mesh (Variables|/Script/Engine.Character|GetMesh _returnvalue))
  (CallFunction|RPCChop)
  (Components|Animation|PlayAnimation _mesh "/Game/Anim/BeaverAnimBite.BeaverAnimBite" false)
  (Utilities|FlowControl|Delay 1.0)
  (Components|Animation|PlayAnimation _mesh "/Game/Anim/BeaverAnim.BeaverAnim" true))

(event Custom|RPC_Chop
  (bind _returnvalue (Components|GetOwner))
  (bind _returnvalue_2 (Transformation|GetActorLocation _returnvalue))
  (bind _outhit (Collision|LineTraceByChannel _returnvalue_2 (+ _returnvalue_2 (* (Transformation|GetActorForwardVector _returnvalue) (Variables|Default|GetChopRange))) "TraceTypeQuery1" false 0 "ForDuration" true "(R=0.000000,G=0.128884,B=1.000000,A=1.000000)" "(R=1.000000,G=0.992607,B=0.000000,A=1.000000)" 1.0))
  (bind _asbp_base_tree (Utilities|Casting|CastToBP_BaseTree (.hitactor _outhit)))
  (Game|Damage|ApplyDamage _asbp_base_tree (Variables|Default|GetChopDamage) 0 (Components|GetOwner))
  (Game|SpawnActorfromClass "/Game/PlayerController/BP_Chip.BP_Chip_C" (Math|Transform|MakeTransform (.location _outhit) "0, 0, 0" "1.000000,1.000000,1.000000") "Undefined" "MultiplyWithRoot" 0 0))

(event Input|EnhancedActionEvents|EnhancedInputActionIA_Bite
  (params (ActionValue :type Boolean) (ElapsedSeconds :type Float%20%28double-precision%29) (TriggeredSeconds :type Float%20%28double-precision%29) (InputAction :type Input%20Action%20Object%20Reference :default "/Game/PlayerController/InputActions/IA_Bite.IA_Bite"))
  (:Started
    (if (Variables|Default|GetCanChop) :!label _label
      (Variables|Default|SetCanChop false)
      (CallFunction|RPCServerChop)
      (Utilities|FlowControl|Delay 1.0)
      (Variables|Default|SetCanChop true)))
  (:Ongoing
    (goto _label)))