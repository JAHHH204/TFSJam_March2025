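; AC_TailSlam provides a tail slam area attack around the player character, with a short cooldown.
; Tick caches the location of player character 0 as the attack's center.
; TailSlamEvent runs a stationary, debug-drawn sphere trace there, ignoring "World"-tagged actors, and applies damage to the single returned hit actor.
; A CanSlam flag and a Delay block repeat slams until the cooldown ends.
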(event Custom|TailSlamEvent
  (bind _location (Variables|Default|GetLocation))
  ;[1 1 1] Tail Slam Event
  (if (Variables|Default|GetCanSlam)
    (Variables|Default|SetCanSlam false)
    (bind _outactors (Actor|GetAllActorswithTag "World"))
    (bind _outhit (Collision|SphereTraceByChannel _location _location 2e+02 "TraceTypeQuery1" false _outactors "ForDuration"))
    (Game|Damage|ApplyDamage (.hitactor _outhit) 1.0 0 0)
    (Utilities|FlowControl|Delay 1.0)
    (Variables|Default|SetCanSlam true)))

(event EventBeginPlay)

(event EventTick
  (params (DeltaSeconds :type Float%20%28single-precision%29))
  ;[1 1 1] Tick
  (Variables|Default|SetLocation (Transformation|GetActorLocation (Game|GetPlayerCharacter 0))))