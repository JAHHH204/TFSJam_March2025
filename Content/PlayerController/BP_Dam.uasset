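; BP_Dam is a dam actor that builds up visually as little trees are brought into it.
; BeginPlay fills an ordered array of its log components.
; When a BP_LittleTree overlaps the Box, the dam clears the tree's player dragging, destroys it, and reveals the next log by advancing an index.
; Trees arriving after all logs are shown are still destroyed.
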(event OnComponentBeginOverlap(Box)
  (params (OverlappedComponent :type Primitive%20Component%20Object%20Reference) (OtherActor :type Actor%20Object%20Reference) (OtherComp :type Primitive%20Component%20Object%20Reference) (OtherBodyIndex :type Integer) (bFromSweep :type Boolean) (SweepResult :type Hit%20Result%20Structure%20%28by%20ref%29))
  (bind _logarray (Variables|Default|GetLogArray))
  (bind _asbp_little_tree (Utilities|Casting|CastToBP_LittleTree OtherActor))
  (Default|RemovePlayerDragging _asbp_little_tree)
  (Actor|DestroyActor _asbp_little_tree)
  (if (Utilities|Array|IsValidIndex _logarray (Variables|Default|GetIndex))
    (Rendering|SetVisibility (Utilities|Array|Get(acopy) _logarray (Variables|Default|GetIndex)) true true)
    (Variables|Default|SetIndex (+ (Variables|Default|GetIndex) 1))))

(event EventBeginPlay
  (Variables|Default|SetLogArray (Utilities|Array|MakeArray (Variables|Default|GetLog1) (Variables|Default|GetLog2) (Variables|Default|GetLog3) (Variables|Default|GetLog4) (Variables|Default|GetLog5) (Variables|Default|GetLog6) (Variables|Default|GetLog7) (Variables|Default|GetLog8) (Variables|Default|GetLog9) (Variables|Default|GetLog11) (Variables|Default|GetLog12) (Variables|Default|GetLog13) (Variables|Default|GetLog14) (Variables|Default|GetLog15) (Variables|Default|GetLog16) (Variables|Default|GetLog17) (Variables|Default|GetLog18) (Variables|Default|GetLog19) (Variables|Default|GetLog20) (Variables|Default|GetLog21))))

(event Collision|EventActorBeginOverlap
  (params (OtherActor :type Actor%20Object%20Reference)))

(event EventTick
  (params (DeltaSeconds :type Float%20%28single-precision%29)))

(fn ConstructionScript)